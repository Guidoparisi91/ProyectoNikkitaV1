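; BP_Nikkita is the player character, moving along a side-view axis and surviving on an oxygen reserve.
; Enhanced Input drives movement, jump and quit, with control yaw flipped by the sign of X acceleration.
; Looping timers drain and print O2, external events damage or restore it, and Tick reloads MAPA2PN when it empties.
; Muerte teleports to a given respawn and refills O2, while TerminaNivel prints success and restarts the map.
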(event `self.ReceiveTick`
  (params (DeltaSeconds :type "Float (single-precision)"))
  (if (<= (`self.O2`) 0.0)
    (`KismetSystemLibrary.PrintString` "SE QUEDO SIN OXIGENO: MUERTE" true true (struct :`R` 1.0 :`B` 0.073311 :`A` 1.0))
    (`GameplayStatics.OpenLevel` "MAPA2PN")))

(event `self.ReceiveBeginPlay`
  (bind _asplayer_controller (cast `PlayerController` (`self.GetController`)))
  (message `EnhancedInputSubsystemInterface.AddMappingContext` (pcsubsystem `EnhancedInputLocalPlayerSubsystem` _asplayer_controller) "/Game/Inputs/MappingContext/IMC_PersonajeInputs.IMC_PersonajeInputs" 0 (struct))
  ;[1 1 1] Pierde Oxigeno y muestra el Oxigeno que le queda
  (`KismetSystemLibrary.K2_SetTimer` null "Pierde O2" 0.5 true)
  (`KismetSystemLibrary.K2_SetTimerDelegate` (delegate `MostrarO2`) 3.0 true))

(event `MostrarO2`
  ;[1 1 1] Pierde Oxigeno y muestra el Oxigeno que le queda
  (`KismetSystemLibrary.PrintString` (`KismetStringLibrary.Concat_StrStr` "Oxigeno que le queda \n" (`KismetStringLibrary.Conv_DoubleToString` (`self.O2`)))))

(event `EnhancedInput|/Game/Inputs/InputsActions/IA_Movimiento`
  (params (ActionValue :type "Float (double-precision)") (ElapsedSeconds :type "Float (double-precision)") (TriggeredSeconds :type "Float (double-precision)") (InputAction :type "InputAction Object Reference" :default "/Game/Inputs/InputsActions/IA_Movimiento.IA_Movimiento"))
  (bind _returnvalue_x (`KismetMathLibrary.BreakVector` (`CharacterMovementComponent.GetCurrentAcceleration` (`self.CharacterMovement`))))
  (:`Triggered`
    (`self.AddMovementInput` (`self.VelMov`) ActionValue)
    (`/Engine/EditorBlueprintResources/StandardMacros.CompareFloat` _returnvalue_x
      (:`>`
        (`Controller.SetControlRotation` (`self.GetController`) (`KismetMathLibrary.MakeRotator` 0.0)))
      (:`<`
        (`Controller.SetControlRotation` (`self.GetController`) (`KismetMathLibrary.MakeRotator` 0.0 0.0 180.0))))))

(event `EnhancedInput|/Game/Inputs/InputsActions/IA_Saltar`
  (params (ActionValue :type "Vector2D Structure") (ElapsedSeconds :type "Float (double-precision)") (TriggeredSeconds :type "Float (double-precision)") (InputAction :type "InputAction Object Reference" :default "/Game/Inputs/InputsActions/IA_Saltar.IA_Saltar"))
  (:`Triggered`
    (`self.Jump`)))

(event `/Game/Interfaces/BPI_Daño.DañoDeNube`
  (params (`DañoNube` :type "Float (double-precision)"))
  (set `self.O2` (- (`self.O2`) `DañoNube`))
  (`KismetSystemLibrary.PrintString` "Pierde O2"))

(event `/Game/Interfaces/BPI_TerminaNivel.TerminaNivel`
  (`KismetSystemLibrary.PrintString` "Sobreviviste!" true true (struct :`G` 1.0 :`B` 0.12266 :`A` 1.0))
  (`GameplayStatics.SetGamePaused` (`self.JuegoEnPausa?`))
  (`KismetSystemLibrary.PrintString` "Comienza De Nuevo!" true true (struct :`R` 0.951642 :`G` 0.07761 :`B` 1.0 :`A` 1.0))
  (`GameplayStatics.SetGamePaused` false)
  (`GameplayStatics.OpenLevel` "MAPA2PN"))

(event `/Game/Interfaces/BPI_RecuperaO2.RecuperaO2`
  (params (CantidadO2Recibe :type "Float (double-precision)"))
  (set `self.O2` (+ CantidadO2Recibe (`self.O2`)))
  (`KismetSystemLibrary.PrintString` "Recupera O2"))

(event `/Game/Interfaces/BPI_Muere.Muerte`
  (params (Respawn :type "Vector Structure"))
  (`KismetSystemLibrary.PrintString` "MUERTE" true true (struct :`R` 1.0 :`G` 0.058806 :`B` 0.009047 :`A` 1.0))
  (`self.K2_SetActorLocation` Respawn)
  (set `self.O2` 100.0))

(event `EnhancedInput|/Game/Inputs/InputsActions/IA_Quit`
  (params (ActionValue :type "Vector2D Structure") (ElapsedSeconds :type "Float (double-precision)") (TriggeredSeconds :type "Float (double-precision)") (InputAction :type "InputAction Object Reference" :default "/Game/Inputs/InputsActions/IA_Quit.IA_Quit"))
  (:`Triggered`
    (`KismetSystemLibrary.QuitGame` null "Quit")))

(fn `Pierde O2`
  (set `self.O2` (- (`self.O2`) 2.0)))

(fn `UserConstructionScript`)