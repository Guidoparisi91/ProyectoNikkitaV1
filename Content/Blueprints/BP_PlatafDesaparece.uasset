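; BP_PlatafDesaparece is a 2D sprite platform that disappears after being touched and returns later.
; When the Overlap component is entered, a short delay precedes hiding the PaperSprite and disabling collision on Overlap and Fisica, guarded by the PlataformaActiva flag.
; End overlap starts a longer delay that restores visibility and collision and clears the flag.
; An alternative blinking sequence is left unconnected.
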(event `self.Fisica.OnComponentBeginOverlap`
  (params (OverlappedComponent :type "PrimitiveComponent Object Reference") (OtherActor :type "Actor Object Reference") (OtherComp :type "PrimitiveComponent Object Reference") (OtherBodyIndex :type Integer) (bFromSweep :type Boolean) (SweepResult :type "HitResult Structure (by ref)")))

(event `self.Overlap.OnComponentBeginOverlap`
  (params (OverlappedComponent :type "PrimitiveComponent Object Reference") (OtherActor :type "Actor Object Reference") (OtherComp :type "PrimitiveComponent Object Reference") (OtherBodyIndex :type Integer) (bFromSweep :type Boolean) (SweepResult :type "HitResult Structure (by ref)"))
  ;[1 1 1] Esto hace que la plataforma desaparezca una ves accionada y vuelva luego de un tiempo
  (if (not (`self.PlataformaActiva`))
    (`KismetSystemLibrary.Delay` 0.5)
    (`PrimitiveComponent.SetCollisionEnabled` (`self.Overlap`) "NoCollision")
    (`PrimitiveComponent.SetCollisionEnabled` (`self.Fisica`) "NoCollision")
    (`SceneComponent.SetVisibility` (`self.PaperSprite`) false false)
    (set `self.PlataformaActiva` true)))

(event `self.Overlap.OnComponentEndOverlap`
  (params (OverlappedComponent :type "PrimitiveComponent Object Reference") (OtherActor :type "Actor Object Reference") (OtherComp :type "PrimitiveComponent Object Reference") (OtherBodyIndex :type Integer))
  ;[1 1 1] Esto hace que la plataforma desaparezca una ves accionada y vuelva luego de un tiempo
  (`KismetSystemLibrary.Delay` 5.0)
  (`PrimitiveComponent.SetCollisionEnabled` (`self.Overlap`) "QueryAndPhysics")
  (`PrimitiveComponent.SetCollisionEnabled` (`self.Fisica`) "QueryAndPhysics")
  (`SceneComponent.SetVisibility` (`self.PaperSprite`) true false)
  (set `self.PlataformaActiva` false))

(fn `UserConstructionScript`)